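; Game mode for a rhythm game that sets up joining players and runs a song from a media playlist.
; Each login records the controller, spawns a RhythmCharacter at the target point matching its index, and shows the game menu.
; BeginPlay plays the playlist entry chosen in the game instance and starts a timeline alongside it.
; When the media closes, every RhythmPlayerController returns to the main menu; logout unpossesses the exiting controller.
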(event OnMediaClosed(MediaPlayer)
  ;[1 1 1] Game Finished And Back To Main Menu
  (for _array_element (Variables|Default|GetAllPlayerControllers)
    (bind _asrhythm_player_controller (Utilities|Casting|CastToRhythmPlayerController _array_element))
    (Default|BackMain _asrhythm_player_controller)))

(event Custom|StartGame
  (params (Index :type Integer))
  (bind _mediaplayer (Variables|Default|GetMediaPlayer))
  ;[1 1 1] Play Media And Start Game
  (Class|MediaPlayer|OpenPlaylistIndex _mediaplayer (Variables|Default|GetMediaPlayList) Index)
  (Media|MediaPlayer|Play _mediaplayer :!class /Script/MediaAssets.MediaPlayer)
  (Timeline|Timeline_0 PlayFromStart))

(event EventBeginPlay
  ;[1 1 1] AutoStart Game
  (bind _asrhythm_game_instance (Utilities|Casting|CastToRhythmGameInstance (Game|GetGameInstance)))
  (CallFunction|StartGame (Variables|/Game/Blueprints/AllLevels/RhythmGameInstance.RhythmGameInstance_C|GetPlaylistIndex _asrhythm_game_instance)))

(event EventPostLogin
  (params (NewPlayer :type Player%20Controller%20Object%20Reference))
  ;[1 1 1] Initial PlayerController And Show Menu
  (Utilities|FlowControl|Sequence
    (:then_0
      (bind _returnvalue (Utilities|Array|Add (Variables|Default|GetAllPlayerControllers) NewPlayer))
      (bind _outactors (Actor|GetAllActorsOfClass "/Game/Blueprints/AllLevels/TargetPoints.TargetPoints_C"))
      (Game|SpawnActorfromClass "/Game/Blueprints/Character/RhythmCharacter.RhythmCharacter_C" (Transformation|GetActorTransform (Utilities|Array|Get(acopy) (Variables|/Game/Blueprints/AllLevels/TargetPoints.TargetPoints_C|GetTargetPoints (Utilities|Array|Get(acopy) _outactors)) _returnvalue)) "AlwaysSpawn" 0 0))
    (:then_1
      (Default|ShowGameMenu (.AsRhythm%20Player%20Controller (Utilities|Casting|CastToRhythmPlayerController NewPlayer))))))

(event EventOnLogout
  (params (ExitingController :type Controller%20Object%20Reference))
  ;[1 1 1] Unposs Controller And Character
  (Pawn|UnPossess ExitingController))

(fn ConstructionScript)