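; RhythmGameInstance is the game instance for a rhythm game, handling menu widgets and level switching.
; It lazily creates and caches the game menu and media playlist widgets, showing the mouse cursor only for the playlist.
; Play stores the selected playlist index before opening GameMap, and BackMain removes the game menu before returning to MainMenu.
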(event Custom|Show%20Game%20Menu
  ;[1 1 1] Initial Setup
  (Utilities|IsValid (Variables|Default|GetGameMenu)
    (:Is%20Valid
      _)
    (:Is%20Not%20Valid
      (bind _returnvalue (UserInterface|CreateWidget "/Game/UMGs/GameMenu/GameMenu.GameMenu_C" (Game|GetPlayerController 0)))
      (bind _output_get (Variables|Default|SetGameMenu _returnvalue))))
  (UserInterface|Viewport|AddtoViewport _output_get 0)
  (Variables|/Script/Engine.PlayerController|SetbShowMouseCursor (Game|GetPlayerController 0) false))

(event Custom|BackMain
  ;[1 1 1] Back to MainMenu
  (Widget|RemovefromParent (Variables|Default|GetGameMenu))
  (Game|OpenLevel(byName) "/Game/Maps/MainMenu"))

(event Custom|ShowMediaPlaylist
  ;[1 1 1] Show Player Medialist
  (Utilities|IsValid (Variables|Default|GetMediaPlaylist)
    (:Is%20Valid
      _)
    (:Is%20Not%20Valid
      (bind _returnvalue (UserInterface|CreateWidget "/Game/UMGs/MainMenu/MediaPlaylist.MediaPlaylist_C" (Game|GetPlayerController 0)))
      (Variables|Default|SetMediaPlaylist _returnvalue)))
  (UserInterface|Viewport|AddtoViewport (Variables|Default|GetMediaPlaylist) 0)
  (Variables|/Script/Engine.PlayerController|SetbShowMouseCursor (Game|GetPlayerController 0) true))

(event Custom|Play
  (params (PlaylistIndex :type Integer))
  ;[1 1 1] Play Media
  (Variables|Default|SetPlaylistIndex PlaylistIndex)
  (Game|OpenLevel(byName) "/Game/Maps/GameMap"))