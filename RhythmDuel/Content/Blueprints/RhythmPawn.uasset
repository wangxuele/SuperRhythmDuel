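; RhythmPawn is a rhythm-game pawn that keeps its sprite in time with MediaPlayer playback and responds to Space presses.
; Each Tick, the playback time's fraction over Duration lerps the PaperSprite between the first two RhythmRouters, looping each cycle.
; Space applies a fractional timing test to playback time, plays Sound on a pass and prints the result for debugging.
; A camera look-at toward that moving point is present but unconnected.
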(event EventBeginPlay)

(event Collision|EventActorBeginOverlap
  (params (OtherActor :type Actor%20Object%20Reference)))

(event EventTick
  (params (DeltaSeconds :type Float%20%28single-precision%29))
  (bind _rhythmrouters (Variables|Default|GetRhythmRouters))
  (Transformation|SetWorldLocation (Variables|Default|GetPaperSprite) (Math|Vector|Lerp(Vector) (Transformation|GetActorLocation (Utilities|Array|Get(acopy) _rhythmrouters)) (Transformation|GetActorLocation (Utilities|Array|Get(acopy) _rhythmrouters 1)) (Math|Float|Fraction (/ (Class|KismetMathLibrary|GetTotalMilliseconds (Class|MediaPlayer|GetTime (Variables|Default|GetMediaPlayer))) (Variables|Default|Getduration)))) false false))

(event Input|KeyboardEvents|SpaceBar
  (params (Key :type Key%20Structure :default "AnyKey"))
  (bind _mediaplayer (Variables|Default|GetMediaPlayer))
  (bind _returnvalue (Class|MediaPlayer|GetTime _mediaplayer))
  (bind _returnvalue_2 (Class|KismetMathLibrary|GetTotalMilliseconds _returnvalue))
  (bind _returnvalue_3 (* _returnvalue_2 2e+03))
  (bind _returnvalue_4 (Math|Float|Fraction _returnvalue_3))
  (bind _returnvalue_5 (< _returnvalue_4 0.5))
  (:Pressed
    (Utilities|FlowControl|Sequence
      (:then_0
        (if _returnvalue_5
          (Audio|Components|Audio|Play (Variables|Default|GetSound) 0.0)))
      (:then_1
        (Development|PrintString (Utilities|String|BuildString(Float) (Utilities|String|ToString(Boolean) _returnvalue_5) "" _returnvalue_4) true true "(R=0.000000,G=0.660000,B=1.000000,A=1.000000)" 1e+01)))))

(fn ConstructionScript)