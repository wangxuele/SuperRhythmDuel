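; Rhythm actor that moves its Scene component along the splines of a RhythmBars array as a playhead driven by the RhythmGameMode.
; BeginPlay places the component at the start of the first bar's spline.
; Each Tick, the game mode's bar index selects the spline and its bar progress sets the spline time for the position.
; GetCurrentKey returns the bar's key at the game mode's current bar and key indices.
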(event EventBeginPlay
  (Transformation|SetWorldLocation (Variables|Default|GetScene) (Spline|GetLocationatTime (Variables|/Game/Blueprints/RhythmBar.RhythmBar_C|GetSpline (Utilities|Array|Get(acopy) (Variables|Default|GetRhythmBars))) 0.0 "World" false) false false))

(event Collision|EventActorBeginOverlap
  (params (OtherActor :type Actor%20Object%20Reference)))

(event EventTick
  (params (DeltaSeconds :type Float%20%28single-precision%29))
  (bind _asrhythm_game_mode (Utilities|Casting|CastToRhythmGameMode (Game|GetGameMode)))
  (bind _barindex (Default|GetBarIndex _asrhythm_game_mode))
  (bind _barprocess (Default|GetBarProcess _asrhythm_game_mode))
  (Transformation|SetWorldLocation (Variables|Default|GetScene) (Spline|GetLocationatTime (Variables|/Game/Blueprints/RhythmBar.RhythmBar_C|GetSpline (Utilities|Array|Get(acopy) (Variables|Default|GetRhythmBars) _barindex)) _barprocess "World" false) false false))

(fn ConstructionScript)

(fn GetCurrentKey
  (bind _asrhythm_game_mode (Utilities|Casting|CastToRhythmGameMode (Game|GetGameMode)))
  (bind _barindex (Default|GetBarIndex _asrhythm_game_mode))
  (bind _keyindex (Default|GetKeyIndex _asrhythm_game_mode))
  (return (Utilities|Array|Get(acopy) (Variables|/Game/Blueprints/RhythmBar.RhythmBar_C|GetKeys (Utilities|Array|Get(acopy) (Variables|Default|GetRhythmBars) _barindex)) _keyindex)))