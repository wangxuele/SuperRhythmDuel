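; KeyActor is a Paper2D sprite actor that displays one key symbol: a direction, FocusEnergy, FireBall or Defence.
; UpdateType stores the key type and selects the matching sprite.
; UpdateState stores the key state and switches on it, but no branch leads anywhere, so the red and transparent sprite tints never run.
; The event graph and construction script are empty.
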(event EventBeginPlay)

(event Collision|EventActorBeginOverlap
  (params (OtherActor :type Actor%20Object%20Reference)))

(event EventTick
  (params (DeltaSeconds :type Float%20%28single-precision%29)))

(fn ConstructionScript)

(fn UpdateType
  (params (Type :type KeyType%20Enum))
  (bind _output_get (Variables|Default|SetKeyType Type))
  (Rendering|Components|Sprite|SetSprite (Variables|Default|GetPaperSprite) (Utilities|Select :Index _output_get :NewEnumerator7 0 :NewEnumerator0 0 :NewEnumerator1 0 :NewEnumerator2 0 :NewEnumerator3 0 :NewEnumerator4 0 :NewEnumerator5 0 :NewEnumerator6 0))
  (return))

(fn UpdateState
  (params (KeyState :type KeyState%20Enum))
  (bind _output_get (Variables|Default|SetKeyState KeyState))
  (switch Utilities|FlowControl|Switch|SwitchonKeyState _output_get))