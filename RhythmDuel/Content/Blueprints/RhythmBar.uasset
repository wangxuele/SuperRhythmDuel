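; RhythmBar is a Blueprint that lays out a bar of rhythm key actors along a spline.
; UpdateBar calls SpawnKeys, then passes each BarData key entry to the matching actor's UpdateType.
; SpawnKeys spawns six KeyActors at evenly stepped spline times, slightly lowered in Z.
; It clears the Keys array first but does not destroy previously spawned actors.
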(event EventBeginPlay)

(event Collision|EventActorBeginOverlap
  (params (OtherActor :type Actor%20Object%20Reference)))

(event EventTick
  (params (DeltaSeconds :type Float%20%28single-precision%29)))

(fn ConstructionScript)

(fn UpdateBar
  (params (BarData :type Bar%20Data%20Structure))
  (CallFunction|SpawnKeys)
  (for (_array_element _array_index) (Utilities|Struct|BreakBarData BarData)
    (Default|UpdateType (Utilities|Array|Get(acopy) (Variables|Default|GetKeys) _array_index) _array_element)))

(fn SpawnKeys
  (Utilities|Array|Clear (Variables|Default|GetKeys))
  (for _index (range 1 6)
    (bind _returnvalue (Game|SpawnActorfromClass "/Game/Blueprints/KeyActor.KeyActor_C" (Math|Transform|MakeTransform (+ (Spline|GetLocationatTime (Variables|Default|GetSpline) (/ (Math|Conversions|ToFloat(Integer) _index) 8.0) "World" false) "0, 0,-30.000000")) "AlwaysSpawn" 0 0))
    (Utilities|Array|Add (Variables|Default|GetKeys) _returnvalue)))