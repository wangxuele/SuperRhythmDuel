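; Rhythm game character Blueprint that plays flipbook animations for idle, focus energy, fireball, defence and falldown states.
; SwitchAnimation stores the new state, selects its flipbook from the CharacterAnimation set and plays it, looping only Idle.
; When a one-shot flipbook finishes, the character switches back to Idle, with Defence waiting through a short delay first.
; BeginPlay starts the character in Idle.
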(event OnFinishedPlaying(Animation)
  ;[1 1 1] Animation Play Finished
  (switch Utilities|FlowControl|Switch|SwitchonAnimationState (Variables|Default|GetAnimationState)
    (:NewEnumerator0
      _)
    (:NewEnumerator1
      _)
    (:NewEnumerator2
      _)
    (:NewEnumerator3
      (Utilities|FlowControl|Delay 1.0))
    (:NewEnumerator4
      _))
  (CallFunction|SwitchAnimation "NewEnumerator0"))

(event Custom|SwitchAnimation
  (params (NewState :type AnimationState%20Enum))
  (bind _animation (Variables|Default|GetAnimation))
  (bind _characteranimation (Variables|Default|GetCharacterAnimation))
  (bind (_idle _focusenerge _fireball _defence _falldown) (Utilities|Struct|BreakCharacterAnimations _characteranimation))
  ;[1 1 1] Switch Animation
  (bind _output_get (Variables|Default|SetAnimationState NewState))
  (Sprite|SetFlipbook (Variables|Default|GetAnimation) (Utilities|Select :Index _output_get :NewEnumerator0 _idle :NewEnumerator1 _focusenerge :NewEnumerator2 _fireball :NewEnumerator3 _defence :NewEnumerator4 _falldown))
  (switch Utilities|FlowControl|Switch|SwitchonAnimationState (Variables|Default|GetAnimationState)
    (:NewEnumerator0
      (Components|Timeline|SetLooping _animation true))
    (:NewEnumerator1
      (Components|Timeline|SetLooping _animation false :!label _label))
    (:NewEnumerator2
      (goto _label))
    (:NewEnumerator3
      (goto _label))
    (:NewEnumerator4
      (goto _label)))
  (Audio|Components|Audio|Play _animation))

(event EventBeginPlay
  ;[1 1 1] Animation Begin
  (CallFunction|SwitchAnimation "NewEnumerator0"))

(fn ConstructionScript)