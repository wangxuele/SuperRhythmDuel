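; KeyActor is a Paper2D actor that displays a single input key prompt, either an arrow direction or Z, X or C.
; UpdateType stores the key type and selects the matching sprite for it.
; UpdateState reads KeyState and tints the sprite opaque black when Active or fully transparent on Miss.
; The event graph and construction script are empty, so neither update function is called from within this Blueprint.
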(event EventBeginPlay)

(event Collision|EventActorBeginOverlap
  (params (OtherActor :type Actor%20Object%20Reference)))

(event EventTick
  (params (DeltaSeconds :type Float%20%28single-precision%29)))

(fn ConstructionScript)

(fn UpdateType
  (params (Type :type KeyType%20Enum))
  (bind _output_get (Variables|Default|SetKeyType Type))
  (Rendering|Components|Sprite|SetSprite (Variables|Default|GetPaperSprite) (Utilities|Select :Index _output_get :NewEnumerator7 0 :NewEnumerator0 (Variables|Keys|GetUp) :NewEnumerator1 (Variables|Keys|GetDown) :NewEnumerator2 (Variables|Keys|GetLeft) :NewEnumerator3 (Variables|Keys|GetRight) :NewEnumerator4 (Variables|Keys|GetZ) :NewEnumerator5 (Variables|Keys|GetX) :NewEnumerator6 (Variables|Keys|GetC)))
  (return))

(fn UpdateState
  (bind _papersprite (Variables|Default|GetPaperSprite))
  (switch Utilities|FlowControl|Switch|SwitchonKeyState (Variables|Default|GetKeyState)
    (:NewEnumerator4
      (Sprite|SetSpriteColor _papersprite "(R=0.000000,G=0.000000,B=0.000000,A=1.000000)"))
    (:NewEnumerator5
      (Sprite|SetSpriteColor _papersprite "(R=0.000000,G=0.000000,B=0.000000,A=0.000000)"))))