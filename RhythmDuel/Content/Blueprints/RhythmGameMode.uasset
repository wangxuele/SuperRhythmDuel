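; Game mode for a rhythm game that drives a media player playlist and judges key presses against LevelData.
; Playback time is the clock, split into four-second bars of eight key slots, with Tick printing each new slot's expected key.
; While media plays, presses update the Rhythm key's hit or miss state, and hits animate the RhythmPawn.
; Helpers toggle and seek playback, report progress, and fill Rhythm bars from LevelData.
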(event Custom|AnyKeyPressed
  (params (RhythmPlayerController :type Rhythm%20Player%20Controller%20Object%20Reference))
  (bind _rhythm (Variables|Default|GetRhythm))
  (if (Audio|Components|Audio|IsPlaying (Variables|Default|GetMediaPlayer))
    (bind _keyactor (Default|GetCurrentKey (Variables|Default|GetRhythm)))
    (if (Utilities|Enum|Equal(Enum) (Variables|/Game/Blueprints/KeyActor.KeyActor_C|GetKeyState _keyactor) "NewEnumerator3")
      (bind _keytype (CallFunction|GetCurrentKey))
      (bind _asrhythm_pawn (Utilities|Casting|CastToRhythmPawn (Pawn|GetControlledPawn RhythmPlayerController)))
      (switch Utilities|FlowControl|Switch|SwitchonKeyType _keytype
        (:NewEnumerator0
          (if (Game|Player|WasInputKeyJustPressed RhythmPlayerController "Up")
            (Default|UpdateAnimations _asrhythm_pawn "NewEnumerator0" :!label _label)
            (bind _keyactor_2 (Default|GetCurrentKey _rhythm :!label _label_2))
            (Default|UpdateState _keyactor_2 "NewEnumerator4")
            (else
              (bind _keyactor_3 (Default|GetCurrentKey _rhythm :!label _label_3))
              (Default|UpdateState _keyactor_3 "NewEnumerator5"))))
        (:NewEnumerator1
          (if (Game|Player|WasInputKeyJustPressed RhythmPlayerController "Down")
            (goto _label)
            (else
              (goto _label_3))))
        (:NewEnumerator2
          (if (Game|Player|WasInputKeyJustPressed RhythmPlayerController "Left")
            (goto _label)
            (else
              (goto _label_3))))
        (:NewEnumerator3
          (if (Game|Player|WasInputKeyJustPressed RhythmPlayerController "Right")
            (goto _label)
            (else
              (goto _label_3))))
        (:NewEnumerator4
          (if (Game|Player|WasInputKeyJustPressed RhythmPlayerController "Z")
            (Default|UpdateAnimations _asrhythm_pawn "NewEnumerator5")
            (goto _label_2)
            (else
              (goto _label_3))))
        (:NewEnumerator5
          (if (Game|Player|WasInputKeyJustPressed RhythmPlayerController "X")
            (Default|UpdateAnimations _asrhythm_pawn "NewEnumerator1")
            (goto _label_2)
            (else
              (goto _label_3))))
        (:NewEnumerator6
          (if (Game|Player|WasInputKeyJustPressed RhythmPlayerController "C")
            (Default|UpdateAnimations _asrhythm_pawn "NewEnumerator4")
            (goto _label_2)
            (else
              (goto _label_3))))))))

(event EventBeginPlay)

(event EventTick
  (params (DeltaSeconds :type Float%20%28single-precision%29))
  (bind _barindex (CallFunction|GetBarIndex))
  (bind _keyindex (CallFunction|GetKeyIndex))
  (if (or (> _keyindex (Variables|Default|GetCurrentKeyIndex)) (> _barindex (Variables|Default|GetCurrentBarIndex)))
    (Utilities|FlowControl|Sequence
      (:then_0
        (bind _keytype (CallFunction|GetCurrentKey))
        (Development|PrintString (Utilities|String|EnumtoString _keytype)))
      (:then_1
        (Variables|Default|SetCurrentBarIndex _barindex)
        (Variables|Default|SetCurrentKeyIndex _keyindex)))))

(fn ConstructionScript)

(fn ToggleMediaPlayer
  (params (PlaylistIndex :type Integer))
  (bind _mediaplayer (Variables|Default|GetMediaPlayer))
  (bind _mediaplayer_2 (Variables|Default|GetMediaPlayer))
  (bind _returnvalue (== PlaylistIndex (Variables|/Script/MediaAssets.MediaPlayer|GetPlaylistIndex _mediaplayer)))
  (if (Audio|Components|Audio|IsPlaying _mediaplayer)
    (if _returnvalue
      (Sequencer|Player|Pause _mediaplayer_2)
      (return)
      (else
        _))
    (elif _returnvalue
      (if (== (Variables|/Script/MediaAssets.MediaPlayer|GetPlaylistIndex _mediaplayer) 0)
        _
        (else
          (Media|MediaPlayer|Play _mediaplayer_2 :!class /Script/MediaAssets.MediaPlayer)
          (return)))))
  (Class|MediaPlayer|OpenPlaylistIndex _mediaplayer_2 (Variables|Default|GetMediaPlayList) PlaylistIndex))

(fn SeekMediaPlayer
  (params (Process :type Float%20%28single-precision%29))
  (Media|MediaPlayer|Seek (Variables|Default|GetMediaPlayer) (* (Media|MediaPlayer|GetDuration) Process)))

(fn GetMediaPlayerProcess
  (return (/ (Class|KismetMathLibrary|GetTotalMilliseconds (Class|MediaPlayer|GetTime (Variables|Default|GetMediaPlayer))) (Class|KismetMathLibrary|GetTotalMilliseconds (Media|MediaPlayer|GetDuration)))))

(fn UpdateRhythm
  (params (Rhythm :type Rhythm%20Object%20Reference))
  (bind _output_get (Variables|Default|SetRhythm Rhythm))
  (for (_array_element _array_index) (Utilities|Struct|BreakLevelData (Variables|Default|GetLevelData))
    (Default|UpdateBar (Utilities|Array|Get(acopy) (Variables|/Game/Blueprints/Rhythm.Rhythm_C|GetRhythmBars _output_get) _array_index) _array_element)))

(fn GetBarIndex
  (return (/ (Math|Timespan|GetSeconds (Class|MediaPlayer|GetTime (Variables|Default|GetMediaPlayer))) 4)))

(fn GetBarProcess
  (return (Math|Float|Fraction (/ (Class|KismetMathLibrary|GetTotalMilliseconds (Class|MediaPlayer|GetTime (Variables|Default|GetMediaPlayer))) 4e+03))))

(fn GetCurrentKey
  (bind _barindex (CallFunction|GetBarIndex))
  (bind _keyindex (CallFunction|GetKeyIndex))
  (return (Utilities|Array|Get(acopy) (Utilities|Struct|BreakBarData (Utilities|Array|Get(acopy) (Utilities|Struct|BreakLevelData (Variables|Default|GetLevelData)) _barindex)) _keyindex)))

(fn GetKeyIndex
  (bind _barprocess (CallFunction|GetBarProcess))
  (return (Math|Float|Floor (* 8 _barprocess))))