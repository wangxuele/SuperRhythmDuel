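; Table actor that displays a vertically scrolling list of BarActors, apparently still in test form.
; BeginPlay spawns a fixed batch of bars, then UpdateBars attaches them to its Scene and scrolls to the first.
; ScrollTo shows a window of VisiableNumber bars from CurrentIndex, stacking them downward and hiding the rest.
; Tick auto-advances the index about every second as a scroll test, with no wrap at the end.
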(event Custom|ScrollTo
  (params (BarIndex :type Integer))
  ;[1 1 1] Scroll Bar To Visiable or Inviaible
  (Variables|BasicSettings|SetCurrentIndex BarIndex)
  (for (_array_element _array_index) (Variables|BasicSettings|GetBars)
    (if (and (>= (- _array_index (Variables|BasicSettings|GetCurrentIndex)) 0) (< (- _array_index (Variables|BasicSettings|GetCurrentIndex)) (Variables|BasicSettings|GetVisiableNumber)))
      (Rendering|SetVisibility (Variables|/Game/Blueprints/Bar/BarActor.BarActor_C|GetScene _array_element) true false)
      (Transformation|SetRelativeLocation (Variables|/Game/Blueprints/Bar/BarActor.BarActor_C|GetScene _array_element) (* "0, 0,-80.000000" (- _array_index (Variables|BasicSettings|GetCurrentIndex))) false false)
      (else
        (Rendering|SetVisibility (Variables|/Game/Blueprints/Bar/BarActor.BarActor_C|GetScene _array_element) false false)))))

(event Custom|ScrollToNext
  ;[1 1 1] Scroll To Next For Autoscroll
  (bind _output_get (Variables|BasicSettings|SetCurrentIndex (+ (Variables|BasicSettings|GetCurrentIndex) 1)))
  (CallFunction|Scrollto _output_get))

(event Custom|UpdateBars
  (params (Bars :type Array%20of%20Bar%20Actor%20Object%20References))
  ;[1 1 1] Clear Prev Attached Bars And Attach New Bars And Scroll to Begining.
  (Utilities|FlowControl|Sequence
    (:then_0
      (Utilities|Array|Clear (Actor|GetAttachedActors)))
    (:then_1
      (bind _output_get (Variables|BasicSettings|SetBars Bars))
      (for _array_element _output_get
        (Transformation|AttachComponentToComponent _array_element (Variables|Default|GetScene) "None" "KeepRelative" "KeepRelative" "KeepRelative" true)))
    (:then_2
      (CallFunction|Scrollto))))

(event EventBeginPlay
  ;[1 1 1] Initial And Spawn Some Bars
  (for _index (range 0 10)
    (bind _returnvalue (Game|SpawnActorfromClass "/Game/Blueprints/Bar/BarActor.BarActor_C" (Math|Transform|MakeTransform "0, 0, 0" "0,90.000000, 0" "3.000000,1,1.000000") "AlwaysSpawn" 0 0))
    (Rendering|SetVisibility (Variables|/Game/Blueprints/Bar/BarActor.BarActor_C|GetPaperSprite _returnvalue) false false)
    (Utilities|Array|Add (Variables|BasicSettings|GetBars) _returnvalue))
  (CallFunction|UpdateBars (Variables|BasicSettings|GetBars)))

(event EventTick
  (params (DeltaSeconds :type Float%20%28single-precision%29))
  ;[1 1 1] Scroll Test
  (if (> (+ DeltaSeconds (Variables|AnimationSettings|GetScrollTime)) 1.0)
    (Variables|AnimationSettings|SetScrollTime 0.0)
    (CallFunction|ScrolltoNext)
    (else
      (Variables|AnimationSettings|SetScrollTime (+ DeltaSeconds (Variables|AnimationSettings|GetScrollTime))))))

(fn ConstructionScript)