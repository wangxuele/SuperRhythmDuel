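; Bar actor that builds a random key sequence, likely for an input prompt, displayed along a spline.
; GeneratKeys spawns KeyActors with random direction types followed by a final random action type, storing them in Keys.
; UpdateKeys attaches each key to the Scene component and spaces them evenly by spline time, slightly lowered.
; Its intended clearing of previous keys only empties the returned attached-actor array, without detaching or destroying anything.
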(event Custom|UpdateKeys
  (params (Keys :type Array%20of%20Key%20Actor%20Object%20References))
  ;[1 1 1] Clear Prev Keys And Attach New Keys
  (Utilities|FlowControl|Sequence
    (:then_0
      (Utilities|Array|Clear (Actor|GetAttachedActors)))
    (:then_1
      (for (_array_element _array_index) Keys
        (Transformation|AttachComponentToComponent _array_element (Variables|Default|GetScene) "None" "KeepRelative" "KeepRelative" "KeepWorld" false)
        (Transformation|SetWorldLocation (Variables|/Game/Blueprints/Key/KeyActor.KeyActor_C|GetScene _array_element) (+ (Spline|GetLocationatTime (Variables|Default|GetSpline) (* (+ _array_index 1) 0.125) "World" false) "0, 0,-40.000000") false false)))))

(event Custom|GeneratKeys
  (bind _keys (Variables|Default|GetKeys))
  ;[1 1 1] Initial And Spawn Some Keys
  (for _index (range 0 5)
    (if (== _index 5)
      (bind _actionkey (CallFunction|RandomActionKey))
      (Utilities|Array|Add _keys _actionkey)
      (else
        (bind _directionkey (CallFunction|RandomDirectionKey))
        (Utilities|Array|Add _keys _directionkey))))
  (CallFunction|UpdateKeys (Variables|Default|GetKeys)))

(fn ConstructionScript)

(fn RandomDirectionKey
  (bind _returnvalue (Game|SpawnActorfromClass "/Game/Blueprints/Key/KeyActor.KeyActor_C" (Math|Transform|MakeTransform "0, 0, 0") "Undefined" 0 (Utilities|Select :Index (Math|Random|RandomIntegerinRange 0 3) :Option%200 "NewEnumerator0" :Option%201 "NewEnumerator1" :Option%202 "NewEnumerator2" :Option%203 "NewEnumerator3") 0))
  (return _returnvalue))

(fn RandomActionKey
  (bind _returnvalue (Game|SpawnActorfromClass "/Game/Blueprints/Key/KeyActor.KeyActor_C" (Math|Transform|MakeTransform "0, 0, 0") "Undefined" 0 (Utilities|Select :Index (Math|Random|RandomIntegerinRange 0 2) :Option%200 "NewEnumerator4" :Option%201 "NewEnumerator5" :Option%202 "NewEnumerator6") 0))
  (return _returnvalue))